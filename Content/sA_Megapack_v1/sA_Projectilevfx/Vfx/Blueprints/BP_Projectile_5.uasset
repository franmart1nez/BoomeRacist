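; BP_Projectile_5 is a VFX projectile that applies damage on overlap and destroys itself after impact.
; BeginPlay assigns its configurable projectile and hit effect assets.
; A hit or overlap swaps the flight effect for the impact effect, disables collision, removes the light and destroys the actor after a short delay.
; Overlaps skip the shooter's side by matching the Enemy or Player tag against walker or first-person character casts; blocking hits apply no damage.
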(event OnComponentBeginOverlap(Sphere1)
  (params (OverlappedComponent :type Primitive%20Component%20Object%20Reference) (OtherActor :type Actor%20Object%20Reference) (OtherComp :type Primitive%20Component%20Object%20Reference) (OtherBodyIndex :type Integer) (bFromSweep :type Boolean) (SweepResult :type Hit%20Result%20Structure%20%28by%20ref%29))
  (bind (_bblockinghit _binitialoverlap _time _distance _location _impactpoint _normal _impactnormal _physmat _hitactor) (Collision|BreakHitResult SweepResult))
  (bind _hiteffects (Variables|Default|GetHiteffects))
  (if (== (Variables|Default|GetTag) "Enemy")
    (Utilities|Casting|CastToBP_BaseEnemyWalker _hitactor
      (:CastFailed
        _))
    (elif (== (Variables|Default|GetTag) "Player")
      (Utilities|Casting|CastToBP_FirstPersonCharacter _hitactor
        (:CastFailed
          _))))
  (Components|Activation|Deactivate (Variables|Default|GetProjectileEffect))
  (Components|Activation|SetActive _hiteffects true false)
  (Transformation|SetWorldLocation _hiteffects _location false false)
  (Collision|SetCollisionEnabled (Variables|Default|GetSphere1) "NoCollision")
  (Game|Damage|ApplyDamage _hitactor (Variables|Default|GetBase%20Damage) 0 0)
  (Components|DestroyComponent (Variables|Default|GetPointLight))
  (Utilities|FlowControl|Delay 1.0)
  (Actor|DestroyActor))

(event OnComponentHit(Sphere1)
  (params (HitComponent :type Primitive%20Component%20Object%20Reference) (OtherActor :type Actor%20Object%20Reference) (OtherComp :type Primitive%20Component%20Object%20Reference) (NormalImpulse :type Vector :default "0, 0, 0") (Hit :type Hit%20Result%20Structure%20%28by%20ref%29))
  (bind _hiteffects (Variables|Default|GetHiteffects))
  (Components|Activation|Deactivate (Variables|Default|GetProjectileEffect))
  (Components|Activation|SetActive _hiteffects true false)
  (Transformation|SetWorldLocation _hiteffects (.Location (Collision|BreakHitResult Hit)) false false)
  (Collision|SetCollisionEnabled (Variables|Default|GetSphere1) "NoCollision")
  (Components|DestroyComponent (Variables|Default|GetPointLight))
  (Utilities|FlowControl|Delay 1.0)
  (Actor|DestroyActor))

(event EventBeginPlay
  (Class|NiagaraComponent|SetAsset (Variables|Default|GetProjectileEffect) (Variables|Default|GetProjectilefx) true)
  (Class|NiagaraComponent|SetAsset (Variables|Default|GetHiteffects) (Variables|Default|GetHitEffect) true))

(fn ConstructionScript)