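; Base Blueprint for physics-object equipment, built around a TongueMop component and two box components.
; Events toggle TongueMop physics simulation and Pawn collision, while Unequip makes all three components ignore Pawns.
; GetEquipmentType returns a fixed enum entry, and the physics replication update is an empty stub.
; Container overlap handling is mostly vestigial: begin does nothing, end resets the overlapped box's mass scale, and impulse and damping logic is disconnected.
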(event OnComponentEndOverlap(Box)
  (params (OverlappedComponent :type Primitive%20Component%20Object%20Reference) (OtherActor :type Actor%20Object%20Reference) (OtherComp :type Primitive%20Component%20Object%20Reference) (OtherBodyIndex :type Integer))
  (if (Variables|Default|GetContainer?)
    (if (Physics|IsSimulatingPhysics OverlappedComponent "None")
      (Class|PrimitiveComponent|SetAllMassScale OverlappedComponent 1.0))))

(event OnComponentBeginOverlap(Box)
  (params (OverlappedComponent :type Primitive%20Component%20Object%20Reference) (OtherActor :type Actor%20Object%20Reference) (OtherComp :type Primitive%20Component%20Object%20Reference) (OtherBodyIndex :type Integer) (bFromSweep :type Boolean) (SweepResult :type Hit%20Result%20Structure%20%28by%20ref%29))
  (if (Variables|Default|GetContainer?)
    (if (Physics|IsSimulatingPhysics OtherComp "None")
      _)))

(event EventUnequip
  (params (Force :type Vector :default "0, 0, 0"))
  (Collision|SetCollisionResponsetoChannel (Variables|Default|GetTongue_Mop) "ECC_Pawn" "ECR_Ignore"))

(event EventEnable/DisablePhysics
  (params (Enable? :type Boolean))
  (Physics|SetSimulatePhysics (Variables|Default|GetTongue_Mop) Enable?))

(event EventUpdatePhysicsReplication
  (params (Replicates? :type Boolean))
  (CallFunction|UpdatePhysicsReplication Replicates?))

(event EventChangeCollisionPawn
  (params (Collides? :type Boolean))
  (CallFunction|PawnCollision Collides?))

(fn ConstructionScript)

(fn PawnCollision
  (params (Collide? :type Boolean))
  (bind _tongue_mop (Variables|Default|GetTongue_Mop))
  (if Collide?
    (Collision|SetCollisionResponsetoChannel _tongue_mop "ECC_Pawn" "ECR_Block")
    (else
      (Collision|SetCollisionResponsetoChannel _tongue_mop "ECC_Pawn" "ECR_Ignore"))))

(fn UpdatePhysicsReplication
  (params (bInReplicates :type Boolean)))

(fn GetEquipmentType
  (params (PlayerAsking :type BP%20First%20Person%20Character%20Object%20Reference))
  (return "NewEnumerator0"))