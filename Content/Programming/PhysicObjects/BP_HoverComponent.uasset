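; BP_HoverComponent is a scene component that applies a hover spring force to its owner's physics-simulating root primitive.
; BeginPlay caches that root, leaving the component idle if it is not simulating physics.
; Each tick, a debug-drawn Visibility trace along local down measures compression within HoverHeight.
; On a hit, a spring-damper force from Stiffness and compression rate pushes along local up at the component's location, so off-center placement adds torque.
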(event EventBeginPlay
  (bind _asprimitive_component (Utilities|Casting|CastToPrimitiveComponent (Variables|/Script/Engine.Actor|GetRootComponent (Components|GetOwner))))
  (bind _output_get (Variables|Default|SetOwnerRef _asprimitive_component))
  (if (not (Physics|IsSimulatingPhysics _output_get "None"))
    (Variables|Default|SetOwnerRef 0)))

(event EventTick
  (params (DeltaSeconds :type Float%20%28single-precision%29))
  (bind _returnvalue (Transformation|GetWorldLocation))
  (bind _hoverheight (Variables|Default|GetHoverHeight))
  (Variables|Default|GetOwnerRef
    (:then
      (bind (_outhit _returnvalue_2) (Collision|LineTraceByChannel _returnvalue (- _returnvalue (* (Math|Vector|GetUpVector) (Variables|Default|GetHoverHeight))) "TraceTypeQuery1" false (Utilities|Array|MakeArray (Components|GetOwner)) "ForDuration"))
      (if _returnvalue_2
        (Variables|Default|SetHoverForce (+ (* (/ (- (/ (- _hoverheight (.Distance (Collision|BreakHitResult _outhit))) _hoverheight) (Variables|Default|GetPreviousCompression)) (Utilities|Time|GetWorldDeltaSeconds)) (Variables|Default|GetDampeningFactor)) (* (/ (- _hoverheight (.Distance (Collision|BreakHitResult _outhit))) _hoverheight) (Variables|Default|GetStiffness))))
        (Variables|Default|SetPreviousCompression (/ (- _hoverheight (.Distance (Collision|BreakHitResult _outhit))) _hoverheight))
        (Class|PrimitiveComponent|AddForceatLocation (Variables|Default|GetOwnerRef) (* (Math|Vector|GetUpVector) (Variables|Default|GetHoverForce)) (Transformation|GetWorldLocation) "None")))
    (:else)))