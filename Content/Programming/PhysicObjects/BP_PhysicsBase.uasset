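; BP_PhysicsBase is a base physics prop that persists through save games and exposes equipment health, type and ID.
; Async SaveGame and LoadGame messages save its state to the GameInstance and restore transform and velocity, matched by ID or path name.
; Destroyed instanced objects remove their saved entry.
; Events toggle physics and Pawn collision, briefly ignoring pawns on unequip; impact sound, replication and most container overlap logic are disconnected.
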(event OnComponentHit(Sphere)
  (params (HitComponent :type Primitive%20Component%20Object%20Reference) (OtherActor :type Actor%20Object%20Reference) (OtherComp :type Primitive%20Component%20Object%20Reference) (NormalImpulse :type Vector :default "0, 0, 0") (Hit :type Hit%20Result%20Structure%20%28by%20ref%29)))

(event OnComponentEndOverlap(Box)
  (params (OverlappedComponent :type Primitive%20Component%20Object%20Reference) (OtherActor :type Actor%20Object%20Reference) (OtherComp :type Primitive%20Component%20Object%20Reference) (OtherBodyIndex :type Integer))
  (if (Variables|Default|GetContainer?)
    (if (Physics|IsSimulatingPhysics OverlappedComponent "None")
      (Class|PrimitiveComponent|SetAllMassScale OverlappedComponent 1.0))))

(event OnComponentBeginOverlap(Box)
  (params (OverlappedComponent :type Primitive%20Component%20Object%20Reference) (OtherActor :type Actor%20Object%20Reference) (OtherComp :type Primitive%20Component%20Object%20Reference) (OtherBodyIndex :type Integer) (bFromSweep :type Boolean) (SweepResult :type Hit%20Result%20Structure%20%28by%20ref%29))
  (if (Variables|Default|GetContainer?)
    (if (Physics|IsSimulatingPhysics OtherComp "None")
      _)))

(event Custom|LoadGameData
  (bind _id (Variables|Default|GetID))
  (bind _savegamedata (Class|INFSaveState|GetGameData(Message) (Game|GetGameInstance)))
  (Utilities|IsValid _savegamedata
    (:Is%20Valid
      (bind _array_element (Utilities|Array|ForEachLoopwithBreak (Variables|/Game/Programming/SaveGame/BP_SaveGame.BP_SaveGame_C|GetPhysObjectsData _savegamedata) :!label _label)
        (:LoopBody
          (if (Utilities|Enum|Equal(Enum) (.ID (Utilities|Struct|BreakSTR_PhysicsObjects _array_element)) (Utilities|String|SelectString (Class|KismetSystemLibrary|GetPathName self) _id (Utilities|Enum|Equal(Enum) _id "")))
            (CallFunction|LoadPhysData _array_element)
            (goto _label Break)))))))

(event EventBeginPlay
  (|StartListeningforAsyncMessage (Utilities|Struct|MakeAsyncMessageId "(TagName=\"System.SaveGame\")")
    (:then
      (|StartListeningforAsyncMessage (Utilities|Struct|MakeAsyncMessageId "(TagName=\"System.LoadGame\")")
        (:OnMessageReceived
          (CallFunction|LoadGameData))))
    (:OnMessageReceived
      (bind _savedata (CallFunction|SavePhysData))
      (Class|INFSaveState|SavePhysObjectData(Message) (Game|GetGameInstance) true _savedata))))

(event EventEnable/DisablePhysics
  (params (Enable? :type Boolean))
  (Physics|SetSimulatePhysics (Variables|Default|GetSphere) Enable?)
  (Collision|SetCollisionResponsetoChannel (Variables|Default|GetBox) "ECC_Pawn" "ECR_Ignore"))

(event EventUnequip
  (params (Force :type Vector :default "0, 0, 0"))
  (Collision|SetCollisionResponsetoChannel (Variables|Default|GetBox) "ECC_Pawn" "ECR_Ignore")
  (Utilities|FlowControl|Delay 1.0)
  (Collision|SetCollisionResponsetoChannel (Variables|Default|GetBox) "ECC_Pawn" "ECR_Block"))

(event EventUpdatePhysicsReplication
  (params (Replicates? :type Boolean))
  (CallFunction|UpdatePhysicsReplication Replicates?))

(event EventChangeCollisionPawn
  (params (Collides? :type Boolean))
  (CallFunction|PawnCollision Collides?))

(event Game|Damage|EventAnyDamage
  (params (Damage :type Float%20%28single-precision%29) (DamageType :type Damage%20Type%20Object%20Reference) (InstigatedBy :type Controller%20Object%20Reference) (DamageCauser :type Actor%20Object%20Reference))
  (Variables|Default|SetHealth (- (Variables|Default|GetHealth) Damage)))

(event EventLoad
  (CallFunction|LoadGameData))

(event EventEndPlay
  (params (EndPlayReason :type EEndPlayReason%20Enum :default "Destroyed"))
  (switch Utilities|FlowControl|Switch|SwitchonEEndPlayReason EndPlayReason
    (:Destroyed
      (if (Variables|Default|GetInstanced?)
        (Class|INFSaveState|RemovePhysData(Message) (Game|GetGameInstance) (Variables|Default|GetID))))))

(fn ConstructionScript)

(fn PawnCollision
  (params (Collide? :type Boolean))
  (if Collide?
    (Collision|SetCollisionResponsetoChannel (Variables|Default|GetSphere) "ECC_Pawn" "ECR_Block")
    (else
      (Collision|SetCollisionResponsetoChannel (Variables|Default|GetSphere) "ECC_Pawn" "ECR_Ignore"))))

(fn UpdatePhysicsReplication
  (params (bInReplicates :type Boolean)))

(fn SavePhysData
  (bind _self self)
  (bind _id (Variables|Default|GetID))
  (bind _returnvalue (Game|GetCurrentLevelName true))
  (return (Utilities|Struct|MakeSTR_PhysicsObjects (Utilities|String|SelectString (Class|KismetSystemLibrary|GetPathName _self) _id (Utilities|Enum|Equal(Enum) _id "")) (Transformation|GetActorTransform) (Transformation|GetVelocity) (Utilities|ResolveSoftReference (Utilities|GetClass _self)) (Variables|Default|GetDestroyed?) (Variables|Default|GetInstanced?) _returnvalue)))

(fn LoadPhysData
  (params (PhysData :type STR%20Physics%20Objects%20Structure))
  (bind (_id _transform _velocity) (Utilities|Struct|BreakSTR_PhysicsObjects PhysData))
  (Variables|Default|SetID _id)
  (Transformation|SetActorTransform _transform)
  (Physics|SetPhysicsLinearVelocity (Variables|Default|GetSphere) _velocity false "None"))

(fn GetEquipmentHealth
  (return (Variables|Default|GetHealth)))

(fn GetEquipmentType
  (params (PlayerAsking :type BP%20First%20Person%20Character%20Object%20Reference))
  (return "NewEnumerator5"))

(fn GetID
  (return (Variables|Default|GetID)))