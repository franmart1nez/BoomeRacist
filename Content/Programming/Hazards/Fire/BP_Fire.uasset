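; Spreading fire hazard that grows, spawns further fires and can be cleaned away.
; Growth enlarges the fire's bounds and raises its spread chance, then sphere-traces at surrounding boxes to spawn up to a random number of new BP_Fire actors.
; Each Clean call shrinks the fire, destroying it once its overlap volume is small enough.
; A looping timer yaws the fire visual toward the camera, billboard-style.
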(event Custom|BiggerFire
  (bind _firebounds (Variables|Default|GetFireBounds))
  (bind _fireoverlapfire (Variables|Default|GetFireOverlapFire))
  (Transformation|SetWorldScale3D _firebounds (* (Transformation|GetWorldScale _firebounds) 1.3))
  (Variables|Default|SetChanceOfSpreading? (+ (Variables|Default|GetChanceOfSpreading?) 1e+01))
  (CallFunction|SpawnLittleFire)
  (Transformation|SetWorldScale3D _fireoverlapfire (* (Transformation|GetWorldScale _fireoverlapfire) 0.9)))

(event Custom|SpawnLittleFire
  (Variables|Default|SetFiresToStart (Math|Random|RandomIntegerinRange 0 3))
  (for _array_element (Variables|Default|GetBoxArray)
    (if (<= (Math|Random|RandomFloatinRange 1.0 1e+02) (Variables|Default|GetChanceOfSpreading?))
      (if (> (Variables|Default|GetFiresToStart) 0)
        (Collision|SetCollisionResponsetoChannel _array_element "ECC_WorldStatic" "ECR_Overlap")
        (bind _returnvalue (Collision|SphereTraceForObjects (Transformation|GetWorldLocation _array_element) (Transformation|GetWorldLocation _array_element) 1e+01 (Utilities|Array|MakeArray "ObjectTypeQuery1" "ObjectTypeQuery2") false 0 "None"))
        (if _returnvalue
          (Game|SpawnActorfromClass "BP_Fire_C" (Math|Transform|MakeTransform "0, 0, 0" "0, 0, 0" "1.000000,1.000000,1.000000") "Undefined" "MultiplyWithRoot" 0 0)
          (Math|Integer|DecrementInt (Variables|Default|GetFiresToStart)
            (:%20%20
              (Collision|SetCollisionResponsetoChannel _array_element "ECC_WorldStatic" "ECR_Ignore")
              (Collision|SetCollisionResponsetoChannel _array_element "ECC_WorldDynamic" "ECR_Ignore")))))))
  (Variables|Default|SetFiresToStart 0))

(event EventBeginPlay
  (Variables|Default|SetBoxArray (Utilities|Array|MakeArray (Variables|Default|GetBox) (Variables|Default|GetBox1) (Variables|Default|GetBox2) (Variables|Default|GetBox3) (Variables|Default|GetBox4) (Variables|Default|GetBox5) (Variables|Default|GetBox10) (Variables|Default|GetBox8) (Variables|Default|GetBox9) (Variables|Default|GetBox11) (Variables|Default|GetBox6) (Variables|Default|GetBox7)))
  (Utilities|Time|SetTimerbyEvent (EventDispatchers|CreateEvent :!event Custom|BiggerFire) 4.0 true true 1.0)
  (Utilities|Time|SetTimerbyFunctionName 0 "FacePlayer" 0.15 true true))

(event EventClean
  (bind _firebounds (Variables|Default|GetFireBounds))
  (bind _fireoverlapfire (Variables|Default|GetFireOverlapFire))
  (Transformation|SetWorldScale3D _firebounds (* (Transformation|GetWorldScale _firebounds) 0.9))
  (Transformation|SetWorldScale3D _fireoverlapfire (* (Transformation|GetWorldScale _fireoverlapfire) 0.9))
  (if (<= (.x (Transformation|GetWorldScale (Variables|Default|GetFireOverlapFire))) 0.4)
    (Actor|DestroyActor)))

(fn ConstructionScript)

(fn FacePlayer
  (bind _fire (Variables|Default|GetFire))
  (Transformation|SetWorldRotation _fire (Math|Rotator|MakeRotator 0.0 0.0 (- (.yaw (Math|Rotator|FindLookatRotation (Transformation|GetWorldLocation _fire) (Camera|GetCameraLocation (Game|GetPlayerCameraManager 0)))) 9e+01)) false false))

(fn GetEquipmentHealth
  (return 0.0))

(fn GetEquipmentType
  (params (PlayerAsking :type BP%20First%20Person%20Character%20Object%20Reference))
  (return "NewEnumerator5"))