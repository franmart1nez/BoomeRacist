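; Base walking enemy drawn as a camera-facing flipbook sprite, driven by BT_Enemy through BP_EnemyAIController.
; Tick yaws the sprite toward the camera and picks a directional flipbook from the player's angle, unless attacking, hit or dying.
; Melee sphere-traces once or repeatedly, while ranged attacks spawn projectiles.
; Damage turns it hostile and plays hit or death flipbooks; death alerts all walkers, and timed burn and wet status are supported.
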(event Custom|MeleeAttack
  (bind _arrow1 (Variables|Default|GetArrow1))
  (bind _returnvalue (Transformation|GetWorldLocation _arrow1))
  ;[0.15 0.15 0.15 0.5] Punch Click Mouse
  (if (not (Variables|Default|GetAttacking?))
    (Variables|Default|SetAttacking? true)
    (Sprite|SetFlipbook (Variables|Default|GetEnemyFB) (Variables|Default|GetAttackFB))
    (if (Variables|Default|GetMultipleAttacks?)
      (Variables|/Script/Engine.CharacterMovementComponent|SetMaxWalkSpeed (Variables|Character|GetCharacterMovement) (Variables|Default|GetMaxWalkSpeedAttacking))
      (for _index (range 0 (Variables|Default|GetAttackAmount))
        (bind (_outhits _returnvalue_2) (Collision|MultiSphereTraceByChannel _returnvalue (+ _returnvalue (* (Math|Vector|GetForwardVector _arrow1) 1.5e+02)) 5e+01 "TraceTypeQuery2" false 0 "None"))
        (if _returnvalue_2
          (Audio|PlaySoundatLocation (Variables|Default|GetSoundMelee) (.Location (Math|Transform|BreakTransform (Transformation|GetActorTransform))) "0, 0, 0" 1.0 1.0 0.0 0 0 0 0)
          (for _array_element _outhits
            (Game|Damage|ApplyDamage (.HitActor (Collision|BreakHitResult _array_element)) (Variables|Default|GetBase%20Damage) 0 0))))
      (CallFunction|FinishAttacking :!label _label)
      (else
        (Utilities|FlowControl|Sequence
          (:then_0
            (bind (_outhits_2 _returnvalue_3) (Collision|MultiSphereTraceByChannel _returnvalue (+ _returnvalue (* (Math|Vector|GetForwardVector _arrow1) 1.5e+02)) 5e+01 "TraceTypeQuery2" false 0 "None"))
            (if _returnvalue_3
              (Audio|PlaySoundatLocation (Variables|Default|GetSoundMelee) (.Location (Math|Transform|BreakTransform (Transformation|GetActorTransform))) "0, 0, 0" 1.0 1.0 0.0 0 0 0 0)
              (for _array_element_2 _outhits_2
                (Game|Damage|ApplyDamage (.HitActor (Collision|BreakHitResult _array_element_2)) (Variables|Default|GetBase%20Damage) 0 0))))
          (:then_1
            (goto _label)))))))

(event Custom|RangedAttack
  (bind _returnvalue (Transformation|GetActorTransform))
  (Audio|PlaySoundatLocation (Variables|Default|GetSoundRanged) (.Location (Math|Transform|BreakTransform _returnvalue)) "0, 0, 0" 1.0 1.0 0.0 0 0 0 0)
  (Game|SpawnActorfromClass "/Game/sA_Megapack_v1/sA_Projectilevfx/Vfx/Blueprints/BP_Projectile_5.BP_Projectile_5_C" _returnvalue "AdjustIfPossibleButAlwaysSpawn" "MultiplyWithRoot" 0 "/Game/sA_Megapack_v1/sA_Projectilevfx/Vfx/Fx/Niagara_Systems/NS_Hit7.NS_Hit7" "/Game/sA_Megapack_v1/sA_Projectilevfx/Vfx/Fx/Niagara_Systems/NS_Projectile7.NS_Projectile7" 0.5 "Enemy" 0))

(event Custom|FinishAttacking
  (if (not (Variables|Default|GetDying?))
    (Utilities|FlowControl|Delay (+ (Class|PaperFlipbookComponent|GetFlipbookLength (Variables|Default|GetEnemyFB)) 0.3))
    (Variables|/Script/Engine.CharacterMovementComponent|SetMaxWalkSpeed (Variables|Character|GetCharacterMovement) (Variables|Default|GetDefaultWalkSpeed))
    (Variables|Default|SetAttacking? false)))

(event Custom|BurnDamage
  (Game|Damage|ApplyDamage self 1e+01 0 0))

(event Custom|uPDATEhOSTILE
  (Default|UpdateHostile (Variables|Default|GetEnemyAIController) true))

(event EventBeginPlay
  (bind _asbp_enemy_aicontroller (Utilities|Casting|CastToBP_EnemyAIController (Pawn|GetController)))
  (Variables|Default|SetEnemyAIController _asbp_enemy_aicontroller)
  (AI|RunBehaviorTree _asbp_enemy_aicontroller "/Game/Programming/Enemies/AI/BT_Enemy.BT_Enemy")
  (Utilities|FlowControl|Delay 0.2)
  (Variables|Default|SetDefaultWalkSpeed (Variables|/Script/Engine.CharacterMovementComponent|GetMaxWalkSpeed (Variables|Character|GetCharacterMovement))))

(event Game|Damage|EventAnyDamage
  (params (Damage :type Float%20%28single-precision%29) (DamageType :type Damage%20Type%20Object%20Reference) (InstigatedBy :type Controller%20Object%20Reference) (DamageCauser :type Actor%20Object%20Reference))
  (bind _enemyaicontroller (Variables|Default|GetEnemyAIController))
  (bind _enemyfb (Variables|Default|GetEnemyFB))
  (bind _enemyfb_2 (Variables|Default|GetEnemyFB))
  (bind _returnvalue (Class|PaperFlipbookComponent|GetFlipbookLength _enemyfb_2))
  (bind _output_get (Variables|Default|SetHostile? true))
  (Default|UpdateHostile (Variables|Default|GetEnemyAIController) _output_get)
  (bind _output_get_2 (Variables|Default|SetHealth (- (Variables|Default|GetHealth) Damage)))
  (if (<= _output_get_2 0.0)
    (Pawn|UnPossess _enemyaicontroller)
    (Actor|DestroyActor _enemyaicontroller)
    (Variables|Default|SetDying? true)
    (Audio|PlaySoundatLocation (Variables|Default|GetSoundDeath) (.Location (Math|Transform|BreakTransform (Transformation|GetActorTransform))) "0, 0, 0" 1.0 1.0 0.0 0 0 0 0)
    (Sprite|SetFlipbook _enemyfb (Variables|Default|GetDeathFB))
    (Utilities|FlowControl|Delay (Class|PaperFlipbookComponent|GetFlipbookLength _enemyfb))
    (Rendering|SetVisibility _enemyfb false false)
    (bind _outactors (Actor|GetAllActorsOfClass "BP_BaseEnemyWalker_C"))
    (for _array_element _outactors
      (CallFunction|UPDATEhOSTILE _array_element))
    (Actor|DestroyActor)
    (elif (not (== (Variables|Default|GetHitFB) 0))
      (Variables|Default|SetGettingHit true)
      (Audio|PlaySoundatLocation (Variables|Default|GetSoundHit) (.Location (Math|Transform|BreakTransform (Transformation|GetActorTransform))) "0, 0, 0" 1.0 1.0 0.0 0 0 0 0)
      (Sprite|SetFlipbook _enemyfb_2 (Variables|Default|GetHitFB))
      (Development|PrintString (Utilities|String|ToString(Float) _returnvalue))
      (Utilities|FlowControl|Delay _returnvalue)
      (Variables|Default|SetGettingHit false))))

(event EventTick
  (params (DeltaSeconds :type Float%20%28single-precision%29))
  (Utilities|SpriteFacePlayer
    (:Out
      (Utilities|GetEnemyAngle
        (:Out
          (if (not (Variables|Default|GetAttacking?))
            (if (not (Variables|Default|GetGettingHit))
              (if (not (Variables|Default|GetDying?))
                (Utilities|CalculateFlipBook)))))))))

(event EventBurn
  (bind _returnvalue (Utilities|Time|SetTimerbyEvent (EventDispatchers|CreateEvent :!event Custom|BurnDamage) 0.3 true))
  (Variables|Default|SetBurnDamageTimer _returnvalue))

(event EventStopBurning
  (Utilities|FlowControl|Delay 0.6)
  (Utilities|Time|ClearandInvalidateTimerbyHandle (Variables|Default|GetBurnDamageTimer)))

(event EventGetWet
  (Variables|Default|SetGetWet? true))

(fn ConstructionScript)

(fn IsWet?
  (return (Variables|Default|GetGetWet?)))