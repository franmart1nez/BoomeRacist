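; AI controller for enemy pawns that turns perception of the player into Blackboard state.
; On BeginPlay it copies the controlled enemy's attack type to the Blackboard.
; Sensing a "Player"-tagged actor sets sight and target keys; losing it clears sight and starts a delay timer, apparently for LostSight, which clears target and hostility.
; Small setter functions wrap each key write, including a player-state setter unused here.
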(event OnTargetPerceptionUpdated(AIPerception)
  (params (Actor :type Actor%20Object%20Reference) (Stimulus :type AI%20Stimulus%20Structure))
  (bind _output_get (Variables|Default|SetPerceivedActor Actor))
  (if (Actor|ActorHasTag _output_get "Player")
    (if (.bSuccessfullySensed (Utilities|Struct|BreakAIStimulus Stimulus))
      (Utilities|Time|ClearandInvalidateTimerbyHandle (Variables|Default|GetLostSightTimer))
      (CallFunction|UpdateSightKey true)
      (CallFunction|UpdateTargetKey (Variables|Default|GetPerceivedActor))
      (else
        (bind _returnvalue (Utilities|Time|SetTimerbyEvent (EventDispatchers|CreateEvent :!event Custom|LostSight) 4.0 false false 4.0))
        (Variables|Default|SetLostSightTimer _returnvalue)
        (CallFunction|UpdateSightKey false)))))

(event Custom|LostSight
  (CallFunction|UpdateTargetKey)
  (CallFunction|UpdateHostile false))

(event EventBeginPlay
  (bind _asbp_enemy_pawn_base (Utilities|Casting|CastToBP_EnemyPawnBase (Pawn|GetControlledPawn)))
  (Variables|Default|SetControlledEnemy _asbp_enemy_pawn_base)
  (CallFunction|UpdateAttackType (Variables|/Game/Programming/Enemies/BP_EnemyPawnBase.BP_EnemyPawnBase_C|GetAttackType _asbp_enemy_pawn_base)))

(fn ConstructionScript)

(fn UpdateSightKey
  (params (CanSeeTarget :type Boolean))
  (AI|Components|Blackboard|SetValueasBool (AI|GetBlackboard 0) (Utilities|Name|MakeLiteralName "CanSeeTarget") CanSeeTarget))

(fn UpdateTargetKey
  (params (TargetActor :type Actor%20Object%20Reference))
  (AI|Components|Blackboard|SetValueasObject (AI|GetBlackboard 0) (Utilities|Name|MakeLiteralName "TargetActor") TargetActor))

(fn UpdateAttackType
  (params (AttackType :type Byte))
  (AI|Components|Blackboard|SetValueasEnum (AI|GetBlackboard 0) (Utilities|Name|MakeLiteralName "EnemyAttackType") AttackType))

(fn UpdateHostile
  (params (Hostile? :type Boolean))
  (AI|Components|Blackboard|SetValueasBool (AI|GetBlackboard 0) (Utilities|Name|MakeLiteralName "Hostile?") Hostile?))

(fn UpdatePlayerActiveState
  (params (PlayerActiveState :type Byte))
  (AI|Components|Blackboard|SetValueasEnum (AI|GetBlackboard 0) (Utilities|Name|MakeLiteralName "PlayerActiveState") PlayerActiveState))