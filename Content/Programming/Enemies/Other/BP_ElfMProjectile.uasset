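; Explosive enemy projectile shown as a flipbook sprite that turns on yaw every tick to face the player.
; BeginPlay sizes the capsule from variables, then sets its main collision channels to overlap after a short delay.
; On overlap it fires a radial impulse, damages a Player-tagged actor, and runs a debug-drawn sphere trace for splash damage.
; Only when that trace hits does it disable collision, hide the sprite and destroy itself after a delay.
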(event OnComponentBeginOverlap(Capsule)
  (params (OverlappedComponent :type Primitive%20Component%20Object%20Reference) (OtherActor :type Actor%20Object%20Reference) (OtherComp :type Primitive%20Component%20Object%20Reference) (OtherBodyIndex :type Integer) (bFromSweep :type Boolean) (SweepResult :type Hit%20Result%20Structure%20%28by%20ref%29))
  (bind _returnvalue (Transformation|GetActorLocation))
  (Class|RadialForceComponent|FireImpulse (Variables|Default|GetRadialForce))
  (if (== (Utilities|Array|Get(acopy) (Variables|/Script/Engine.Actor|GetTags OtherActor)) "Player")
    (Game|Damage|ApplyDamage OtherActor 25.0 0 0))
  (bind (_outhits _returnvalue_2) (Collision|MultiSphereTraceForObjects _returnvalue _returnvalue 5e+02 (Utilities|Array|MakeArray "ObjectTypeQuery3" "ObjectTypeQuery9") false 0 "ForDuration"))
  (if _returnvalue_2
    (for _array_element _outhits
      (Game|Damage|ApplyDamage (.HitActor (Collision|BreakHitResult _array_element)) 1e+01 0 0))
    (Collision|SetCollisionEnabled (Variables|Default|GetCapsule) "NoCollision")
    (Rendering|SetVisibility (Variables|Default|GetPaperFlipbook) false false)
    (Utilities|FlowControl|Delay 3.0)
    (Actor|DestroyActor)))

(event Custom|HoverFacePlayer
  (bind _paperflipbook (Variables|Default|GetPaperFlipbook))
  ;[0.15 0.15 0.15 0.5] Hover Face Player
  (Transformation|SetWorldRotation _paperflipbook (Math|Rotator|MakeRotator 0.0 9e+01 (- (.yaw (Math|Rotator|FindLookatRotation (Transformation|GetWorldLocation _paperflipbook) (Transformation|GetActorLocation (Game|Player|GetPlayerPawn 0)))) 9e+01)) false false))

(event EventBeginPlay
  (bind _capsule (Variables|Default|GetCapsule))
  (Sprite|SetFlipbook (Variables|Default|GetPaperFlipbook) (Variables|Default|GetNew%20Flipbook))
  (Components|Capsule|SetCapsuleRadius _capsule (Variables|Default|GetRadius) true)
  (Components|Capsule|SetCapsuleHalfHeight _capsule (Variables|Default|GetHalf%20Height) true)
  (Collision|IgnoreActorwhenMoving (Variables|Default|GetCapsule) (Variables|Default|GetActorIgnoreCollision) false)
  (Utilities|FlowControl|Delay 0.2)
  (Collision|SetCollisionResponsetoChannel (Variables|Default|GetCapsule) "ECC_WorldStatic" "ECR_Overlap")
  (Collision|SetCollisionResponsetoChannel (Variables|Default|GetCapsule) "ECC_WorldDynamic" "ECR_Overlap")
  (Collision|SetCollisionResponsetoChannel (Variables|Default|GetCapsule) "ECC_Pawn" "ECR_Overlap")
  (Collision|SetCollisionResponsetoChannel (Variables|Default|GetCapsule) "ECC_PhysicsBody" "ECR_Overlap"))

(event EventTick
  (params (DeltaSeconds :type Float%20%28single-precision%29))
  (CallFunction|HoverFacePlayer))

(fn ConstructionScript)