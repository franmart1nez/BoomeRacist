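; BP_ElfM is an elf enemy that grabs a random nearby comrade and hurls it at the player.
; GetPrey switches to async-loaded hover and attack flipbooks while a timeline lerps the victim to the grab point.
; The victim is then replaced by a BP_ElfMProjectile copying its hover flipbook and capsule size.
; After a delay, Throw enables physics on the projectile and applies an impulse toward PlayerTarget, scaled by distance.
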(event Custom|Throw
  (params (New%20Flipbook :type Paper%20Flipbook%20Object%20Reference) (Radius :type Float%20%28single-precision%29) (Half%20Height :type Float%20%28single-precision%29))
  (bind _playertarget (Variables|Default|GetPlayerTarget))
  (bind _returnvalue (Transformation|GetActorLocation _playertarget))
  (bind _returnvalue_2 (Game|SpawnActorfromClass "/Game/Programming/Enemies/Other/BP_ElfMProjectile.BP_ElfMProjectile_C" (Math|Transform|MakeTransform (Transformation|GetWorldLocation (Variables|Default|GetGrabLocation)) "0.000000,0.000000,90.000000" "1.000000,1.000000,1.000000") "Undefined" "MultiplyWithRoot" 0 New%20Flipbook Radius Half%20Height self 0))
  (Collision|IgnoreActorwhenMoving (Variables|Default|GetCapsuleComponent) _returnvalue_2 false)
  (Utilities|FlowControl|Delay 3.0)
  (Sprite|SetFlipbook (Variables|Default|GetEnemyFB) (Variables|Default|GetAttackHover))
  (Physics|SetSimulatePhysics (Variables|/Game/Programming/Enemies/Other/BP_ElfMProjectile.BP_ElfMProjectile_C|GetCapsule _returnvalue_2) true)
  (Physics|AddImpulse (Variables|/Game/Programming/Enemies/Other/BP_ElfMProjectile.BP_ElfMProjectile_C|GetCapsule _returnvalue_2) (* (Math|Vector|GetUnitDirection(Vector) _returnvalue (Transformation|GetWorldLocation (Variables|/Game/Programming/Enemies/Other/BP_ElfMProjectile.BP_ElfMProjectile_C|GetCapsule _returnvalue_2))) (* (* (Math|Vector|Distance(Vector) _returnvalue (Transformation|GetWorldLocation (Variables|/Game/Programming/Enemies/Other/BP_ElfMProjectile.BP_ElfMProjectile_C|GetCapsule _returnvalue_2))) 3e+02) -1.0)) "None" false)
  (Utilities|FlowControl|Delay (Class|PaperFlipbookComponent|GetFlipbookLength (Variables|Default|GetEnemyFB)))
  (Variables|Default|SetGrabbedEnemy? false)
  (Variables|Default|SetHovering? false))

(event Custom|GetPrey
  (bind _closecomrades (Variables|Default|GetCloseComrades))
  (bind _returnvalue (Utilities|Array|Length _closecomrades))
  (bind _returnvalue_2 (- _returnvalue 1))
  (bind _returnvalue_3 (Math|Random|RandomIntegerinRange 0 _returnvalue_2))
  (bind _output (Utilities|Array|Get(acopy) _closecomrades _returnvalue_3))
  (CallFunction|CheckforComrades)
  (if (Utilities|Array|IsNotEmpty _closecomrades)
    (bind _output_get (Variables|Default|SetGrabbedEnemy _output))
    (Variables|/Game/Programming/Enemies/BP_EnemyPawnBase.BP_EnemyPawnBase_C|SetHovering? _output_get true)
    (Default|SetHoverFB _output)
    (Default|DisableAI _output)
    (Variables|Default|SetEnemyHoverFB (Variables|/Game/Programming/Enemies/BP_EnemyPawnBase.BP_EnemyPawnBase_C|GetHoveringFB (Variables|Default|GetGrabbedEnemy)))
    (CallFunction|SetHoveringAttackFB)
    (Variables|Default|SetGrabbedEnemyLocation (Transformation|GetActorLocation _output))
    (bind _grab_alpha (Timeline|Grab PlayFromStart)
      (:Update
        (Transformation|SetActorLocation (Variables|Default|GetGrabbedEnemy) (Math|Vector|Lerp(Vector) (Variables|Default|GetGrabbedEnemyLocation) (Transformation|GetWorldLocation (Variables|Default|GetGrabLocation)) _grab_alpha) false true))
      (:Finished
        (Variables|Default|SetGrabbedEnemy? true)
        (CallFunction|Throw (Variables|Default|GetEnemyHoverFB) (Components|Capsule|GetScaledCapsuleRadius (Variables|/Script/Engine.Character|GetCapsuleComponent (Variables|Default|GetGrabbedEnemy))) (Components|Capsule|GetScaledCapsuleHalfHeight (Variables|/Script/Engine.Character|GetCapsuleComponent (Variables|Default|GetGrabbedEnemy))))
        (Actor|DestroyActor (Variables|Default|GetGrabbedEnemy))
        (Variables|Default|SetGrabbedEnemy 0)))))

(event Custom|SetHoveringAttackFB
  (Variables|Default|SetHovering? true)
  (bind _object (Utilities|AsyncLoadAsset (Variables|Default|GetStartHover))
    (:Completed
      (CallFunction|SetFlipBook _object)
      (bind _object_2 (Utilities|AsyncLoadAsset (Variables|Default|GetAttackFB))
        (:then
          (Utilities|FlowControl|Delay (Class|PaperFlipbookComponent|GetFlipbookLength (Variables|Default|GetEnemyFB)))
          (CallFunction|SetFlipBook _object_2))))))

(event EventBeginPlay
  (|CallParentFunction) ; This node is disabled and will not be called.\nDrag off pins to build functionality.
)

(event Collision|EventActorBeginOverlap
  (params (OtherActor :type Actor%20Object%20Reference)))

(event EventTick
  (params (DeltaSeconds :type Float%20%28single-precision%29))
  (|CallParentFunction DeltaSeconds))

(fn ConstructionScript
  (|CallParentFunction))