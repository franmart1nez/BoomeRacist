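; Dialogue component that runs a conversation between the first-person player and an actor, driven by a StateTree asset.
; StartDialogue stores participants and entry tag, creates the dialogue widget, runs the tree on its owner and optionally switches to dialogue input.
; Widget advance and option events are rebroadcast through component dispatchers.
; EndDialogue re-enables input, clears state and broadcasts outgoing tags, though AddOutgoingTag is an empty stub.
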(fn StartDialogue
  (params (TalkingWith :type Actor%20Object%20Reference) (ActorTalking :type Actor%20Object%20Reference) (DialogueTree :type State%20Tree%20Object%20Reference) (IncomingTag :type Gameplay%20Tag%20Container%20Structure) (DisableCharacterInput? :type Boolean) (EndDialogueDelegate :type Delegate%20%28by%20ref%29))
  (EventDispatchers|BindEventtoOnDialogueEnded EndDialogueDelegate)
  (Utilities|FlowControl|Sequence
    (:then_0
      (Variables|Default|SetTalking%20With TalkingWith)
      (Variables|Default|SetActor%20Talking ActorTalking)
      (Variables|Default|SetCurrentDialogue%20Tree DialogueTree)
      (Variables|Default|SetEntry%20Tag IncomingTag)
      (GameplayTags|AddGameplayTag (Variables|Default|GetEntry%20Tag) (select (GameplayTags|DoesContainerMatchTagQuery IncomingTag (GameplayTags|MakeGameplayTagQuery "(TokenStreamVersion=0,TagDictionary=((TagName=\"Dialogue.EntryPoint\")),QueryTokenStream=(0,1,1,1,0),UserDescription=\"\",AutoDescription=\" ANY( Dialogue.EntryPoint )\")")) "(TagName=\"\")" "(TagName=\"Dialogue.EntryPoint.Default\")") :!class /Script/GameplayTags.BlueprintGameplayTagLibrary))
    (:then_1
      (bind _asbp_first_person_character (Utilities|Casting|CastToBP_FirstPersonCharacter (Variables|Default|GetTalking%20With)))
      (bind _asbp_first_person_player_controller (Utilities|Casting|CastToBP_FirstPersonPlayerController (Pawn|GetController _asbp_first_person_character)))
      (bind _returnvalue (UserInterface|CreateWidget (Variables|Default|GetDialogueScreenWidget) _asbp_first_person_player_controller))
      (bind _output_get (Variables|Default|SetWDG_Dialogue _returnvalue))
      (UserInterface|Viewport|AddtoViewport _output_get 0)
      (Class|GameplayStateTreeBlueprintFunctionLibrary|RunStateTree (Components|GetOwner) (Variables|Default|GetCurrentDialogue%20Tree))
      (EventDispatchers|BindEventtoOnAdvanceDialogue (Variables|Default|GetWDG_Dialogue) (EventDispatchers|CreateEvent :!event AdvanceDialogue))
      (EventDispatchers|BindEventtoOnOptionSelected (Variables|Default|GetWDG_Dialogue) (EventDispatchers|CreateEvent :!event OptionSelected)))
    (:then_2
      (if DisableCharacterInput?
        (bind _asbp_first_person_character_2 (Utilities|Casting|CastToBP_FirstPersonCharacter (Variables|Default|GetTalking%20With)))
        (bind _asbp_first_person_player_controller_2 (Utilities|Casting|CastToBP_FirstPersonPlayerController (Pawn|GetController _asbp_first_person_character_2)))
        (Input|DisableInput _asbp_first_person_character_2 _asbp_first_person_player_controller_2)
        (Input|AddMappingContext (PlayerController|LocalPlayerSubsystems|GetEnhancedInputLocalPlayerSubsystem _asbp_first_person_player_controller_2) "/Game/Programming/InputMapping/Dialogue/IMC_Dialogue.IMC_Dialogue" 0 "(bIgnoreAllPressedKeysUntilRelease=True,bForceImmediately=False,bNotifyUserSettings=False)")
        (Variables|/Script/Engine.PlayerController|SetbShowMouseCursor _asbp_first_person_player_controller_2 true)))))

(fn EndDialogue
  (bind _asbp_first_person_character (Utilities|Casting|CastToBP_FirstPersonCharacter (Variables|Default|GetTalking%20With)))
  (bind _asbp_first_person_player_controller (Utilities|Casting|CastToBP_FirstPersonPlayerController (Pawn|GetController _asbp_first_person_character)))
  (Input|EnableInput _asbp_first_person_character _asbp_first_person_player_controller)
  (Variables|Default|SetTalking%20With 0)
  (Variables|Default|SetActor%20Talking 0)
  (Variables|Default|SetCurrentDialogue%20Tree 0)
  (Variables|Default|SetEntry%20Tag "")
  (Widget|RemovefromParent (Variables|Default|GetWDG_Dialogue))
  (Variables|Default|SetWDG_Dialogue 0)
  (Default|CallOnDialogueEnded (Variables|Default|GetOutgoing%20Tags)))

(fn AdvanceDialogue
  (Default|CallOnDialogueAdvance))

(fn OptionSelected
  (params (OptionIndex :type Integer))
  (Default|CallOnDialogueOptionsSelected OptionIndex))

(fn AddOutgoingTag
  (params (Tag :type Gameplay%20Tag%20Structure)))