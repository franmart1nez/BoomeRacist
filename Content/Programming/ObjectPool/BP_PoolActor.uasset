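; BP_PoolActor is an object pool actor that toggles between in-use and pooled states instead of being spawned and destroyed.
; SetInUse switches collision, visibility and actor tick together, and the actor starts out inactive on BeginPlay.
; Activation restarts a TimeToLive timer, deactivation clears it, and ReturnToPool puts the actor back in the inactive state.
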(event Custom|SetInUse
  (params (InUse :type Boolean))
  (Variables|Default|SetInUse InUse)
  (Collision|SetActorEnableCollision InUse)
  (Rendering|SetActorHiddenInGame (not InUse))
  (Actor|Tick|SetActorTickEnabled InUse)
  (Utilities|Time|ClearandInvalidateTimerbyHandle (Variables|Default|GetSetInUseTimer))
  (if InUse
    (bind _returnvalue (Utilities|Time|SetTimerbyEvent (EventDispatchers|CreateEvent :!event Custom|ReturnToPool) (Variables|Default|GetTimeToLive)))
    (Variables|Default|SetSetInUseTimer _returnvalue)))

(event Custom|ReturnToPool
  (CallFunction|SetinUse false))

(event EventBeginPlay
  (CallFunction|SetinUse false))

(fn ConstructionScript)