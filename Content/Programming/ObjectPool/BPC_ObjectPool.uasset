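; Actor component that implements an object pool, reusing pre-spawned actors of a configurable class.
; On BeginPlay it spawns PoolSize actors at an off-world holding location, passing each a TimeToLive and storing it in the ObjectPool array.
; SpawnFromPool linearly searches for the first actor not in use, moves it to the requested transform and flags it InUse.
; An exhausted pool only prints a message and does not grow.
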(event Custom|InitializePool
  (for _index (range 0 (Variables|Default|GetPoolSize))
    (bind _returnvalue (Game|SpawnActorfromClass (Variables|Default|GetPooledActorClass) (Math|Transform|MakeTransform "-1000.000000,-1000.000000,-1000.000000" "0, 0, 0" "1.000000,1.000000,1.000000") "Undefined" "MultiplyWithRoot" 0 (Variables|Default|GetTime%20to%20Live) 0))
    (Utilities|Array|AddUnique (Variables|Default|GetObjectPool) _returnvalue)))

(event EventBeginPlay
  (CallFunction|InitializePool))

(fn FindFirstAvailableActor
  (for _array_element (Variables|Default|GetObjectPool)
    (if (not (Variables|/Game/Programming/ObjectPool/BP_PoolActor.BP_PoolActor_C|GetInUse _array_element))
      (return _array_element))))

(fn SpawnfromPool
  (params (SpawnTransform :type Transform))
  (bind _pooledactor (CallFunction|FindFirstAvailableActor))
  (Utilities|IsValid _pooledactor
    (:Is%20Valid
      (Transformation|SetActorTransform _pooledactor SpawnTransform)
      (Default|SetinUse _pooledactor true)
      (return _pooledactor))
    (:Is%20Not%20Valid
      (Development|PrintString "No actors in pool"))))