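; Base weapon Blueprint with flipbook-animated flamethrower, melee wiper and regular fire variants, selected by flags.
; Shoot starts a looping auto-fire timer and StopShooting clears it; regular fire here only plays animation.
; The wiper sphere-traces to clean and damage targets, hitting far harder on ones the longer-range alt spray has wet.
; Flamethrower fire toggles an overlap volume that sends burn and stop-burn messages.
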(event OnComponentBeginOverlap(FireDamage)
  (params (OverlappedComponent :type Primitive%20Component%20Object%20Reference) (OtherActor :type Actor%20Object%20Reference) (OtherComp :type Primitive%20Component%20Object%20Reference) (OtherBodyIndex :type Integer) (bFromSweep :type Boolean) (SweepResult :type Hit%20Result%20Structure%20%28by%20ref%29))
  (if (Variables|Default|GetFireThrowerShooting)
    (Class|INFEnemyInterface|Burn(Message) OtherActor)))

(event OnComponentEndOverlap(FireDamage)
  (params (OverlappedComponent :type Primitive%20Component%20Object%20Reference) (OtherActor :type Actor%20Object%20Reference) (OtherComp :type Primitive%20Component%20Object%20Reference) (OtherBodyIndex :type Integer))
  (Class|INFEnemyInterface|StopBurning(Message) OtherActor))

(event Custom|MakeBullets/Fire
  (bind _arrow (Variables|Default|GetArrow))
  (bind _returnvalue (Transformation|GetWorldLocation _arrow))
  (if (Variables|Default|GetMelee?)
    ;[0.15 0.15 0.15 0.5] Melee
    (Sprite|SetFlipbook (Variables|Default|GetWeaponAlt) (Utilities|Array|Get(acopy) (Variables|Default|GetWiperFB) 1))
    (bind (_outhits _returnvalue_2) (Collision|MultiSphereTraceByChannel _returnvalue (+ _returnvalue (* (Math|Vector|GetForwardVector _arrow) 1.5e+02)) 5e+01 "TraceTypeQuery2" false (Utilities|Array|MakeArray (Game|Player|GetPlayerPawn 0)) "ForDuration"))
    (if _returnvalue_2
      (Audio|PlaySound2D "/Game/Programming/SFX/Everything/Weapons/Wiper/wipe.wipe" 1.0 1.0 0.0 "/Game/Programming/NewSoundConcurrency.NewSoundConcurrency" 0)
      (for _array_element _outhits
        (bind _iswet_ (Class|INFEnemyInterface|IsWet?(Message) (.HitActor (Collision|BreakHitResult _array_element))))
        (Class|INFClean|Clean(Message) (.HitActor (Collision|BreakHitResult _array_element)))
        (Game|Damage|ApplyDamage (.HitActor (Collision|BreakHitResult _array_element)) (Math|Float|SelectFloat 1e+03 5.0 _iswet_) 0 0)))
    (elif (Variables|Default|GetFlameThrower?)
      (Components|Activation|Activate (Variables|Default|GetFlame) false)
      (Variables|Default|SetFireThrowerShooting true)
      (Audio|PlaySound2D "/Game/Programming/SFX/Everything/Weapons/pAINTTHROWER/PaintFireLoop.PaintFireLoop" 1.0 1.0 0.0 0 0)
      (Collision|SetCollisionResponsetoAllChannels (Variables|Default|GetFireDamage) "ECR_Overlap")
      (else
        ;[0.15 0.15 0.15 0.5] 'Regular' Shooting
        (Sprite|SetFlipbook (Variables|Default|GetWeaponFB) (Utilities|Array|Get(acopy) (Variables|Default|GetFireFB) (Math|Random|RandomInteger 3)))))))

(event EventBeginPlay)

(event EventShoot
  (bind _weaponfb (Variables|Default|GetWeaponFB))
  (bind _returnvalue (Utilities|Time|SetTimerbyEvent (EventDispatchers|CreateEvent :!event Custom|MakeBullets/Fire) (Variables|Default|GetRateOfFire) true true (Variables|Default|GetInitial%20Start%20Delay)))
  (Variables|Default|SetAutoShootTimer _returnvalue)
  (if (Variables|Default|GetFlameThrower?)
    (Audio|PlaySound2D "/Game/Programming/SFX/Everything/Weapons/pAINTTHROWER/PaintPressTrigger.PaintPressTrigger" 1.0 1.0 0.0 0 0)
    (Sprite|SetFlipbook _weaponfb (Utilities|Array|Get(acopy) (Variables|Default|GetFireFB)))
    (Utilities|FlowControl|Delay (Class|PaperFlipbookComponent|GetFlipbookLength _weaponfb))
    (Sprite|SetFlipbook (Variables|Default|GetWeaponFB) (Utilities|Array|Get(acopy) (Variables|Default|GetFireFB) 1))))

(event EventStopShooting
  (bind _weaponfb (Variables|Default|GetWeaponFB))
  ;[0.15 0.15 0.15 0.5] StopShooting
  (Components|Activation|Deactivate (Variables|Default|GetFlame))
  (Utilities|Time|ClearandInvalidateTimerbyHandle (Variables|Default|GetAutoShootTimer))
  (if (Variables|Default|GetFlameThrower?)
    (Collision|SetCollisionResponsetoAllChannels (Variables|Default|GetFireDamage) "ECR_Ignore")
    (Sprite|SetFlipbook _weaponfb (Utilities|Array|Get(acopy) (Variables|Default|GetFireFB) 2))
    (Utilities|FlowControl|Delay (Class|PaperFlipbookComponent|GetFlipbookLength _weaponfb))
    (Sprite|SetFlipbook (Variables|Default|GetWeaponFB) (Variables|Default|GetIdleFB))
    (elif (Variables|Default|GetAltShoot?)
      (Sprite|SetFlipbook (Variables|Default|GetWeaponAlt) (Utilities|Array|Get(acopy) (Variables|Default|GetWiperFB)))
      (else
        (Sprite|SetFlipbook (Variables|Default|GetWeaponFB) (Variables|Default|GetIdleFB))))))

(event EventInitializeWeapon
  (bind _weaponfb (Variables|Default|GetWeaponFB))
  (Utilities|FlowControl|Sequence
    (:then_0
      (Sprite|SetFlipbook _weaponfb (Variables|Default|GetAppearFB))
      (Utilities|FlowControl|Delay (Class|PaperFlipbookComponent|GetFlipbookLength _weaponfb))
      (Sprite|SetFlipbook (Variables|Default|GetWeaponFB) (Variables|Default|GetIdleFB)))
    (:then_1
      (if (Variables|Default|GetAltShoot?)
        (Sprite|SetFlipbook (Variables|Default|GetWeaponAlt) (Utilities|Array|Get(acopy) (Variables|Default|GetWiperFB)))))))

(event EventAlternativeShoot
  (bind _arrow (Variables|Default|GetArrow))
  (bind _returnvalue (Transformation|GetWorldLocation _arrow))
  ;[0.15 0.15 0.15 0.5] Melee
  (Sprite|SetFlipbook (Variables|Default|GetWeaponFB) (Utilities|Array|Get(acopy) (Variables|Default|GetFireFB) (Math|Random|RandomInteger 3)))
  (bind (_outhits _returnvalue_2) (Collision|MultiSphereTraceByChannel _returnvalue (+ _returnvalue (* (Math|Vector|GetForwardVector _arrow) 5e+02)) 6e+01 "TraceTypeQuery2" false (Utilities|Array|MakeArray (Game|Player|GetPlayerPawn 0)) "ForDuration"))
  (if _returnvalue_2
    (Audio|PlaySound2D "/Game/Programming/SFX/Everything/Weapons/Spreayer/SSpray.SSpray" 1.0 1.0 0.0 "/Game/Programming/NewSoundConcurrency.NewSoundConcurrency" 0)
    (for _array_element _outhits
      (Class|INFEnemyInterface|GetWet(Message) (.HitActor (Collision|BreakHitResult _array_element)))
      (Class|INFClean|WetWindows(Message) (.HitActor (Collision|BreakHitResult _array_element))))))

(fn ConstructionScript)