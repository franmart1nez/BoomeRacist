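; BP_WiperPickup is a weapon pickup actor for the Wiper that turns its display toward the player's camera.
; Each Tick sets the WeaponFB component's world yaw from a look-at rotation to the camera, offset by 90 degrees, keeping pitch and roll at zero.
; Logic to equip BP_Wiper on BP_FirstPersonCharacter and destroy the pickup is present but disconnected, and this graph's overlap event is empty.
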(event EventBeginPlay)

(event Collision|EventActorBeginOverlap
  (params (OtherActor :type Actor%20Object%20Reference)))

(event EventTick
  (params (DeltaSeconds :type Float%20%28single-precision%29))
  (bind _weaponfb (Variables|Default|GetWeaponFB))
  (Transformation|SetWorldRotation _weaponfb (Math|Rotator|MakeRotator 0.0 0.0 (- (.yaw (Math|Rotator|FindLookatRotation (Transformation|GetWorldLocation _weaponfb) (Camera|GetCameraLocation (Game|GetPlayerCameraManager 0)))) 9e+01)) false false))

(fn ConstructionScript)