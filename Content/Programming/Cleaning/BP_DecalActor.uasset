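; Cleanable decal actor that dissolves in increments each time Clean is called.
; Shortly after BeginPlay it creates a dynamic material and, if Shot is valid, traces along four directional arrows against WorldStatic.
; SetRotation applies a random roll, then tilts the decal according to which traces hit nearby surfaces.
; Clean runs a timeline that lerps NewDissolve, whose RepNotify updates the material's Dissolve parameter.
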(event Custom|SetRotation
  (Transformation|AddRelativeRotation (Variables|Default|GetDecal) (Math|Rotator|MakeRotator (Math|Random|RandomFloatinRange 0.0 3.6e+02) 0.0 0.0) false false)
  (if (Math|Boolean|ANDBoolean (Variables|Default|GetHitDown) (not (Variables|Default|GetHitRight)) (not (Variables|Default|GetHitLeft)) (not (Variables|Default|GetHitUp)))
    (Transformation|AddRelativeRotation (Variables|Default|GetDecal) "35.000000,0.000000,0.000000" false false)
    (Development|PrintString "HitDown")
    (elif (Math|Boolean|ANDBoolean (Variables|Default|GetHitDown) (Variables|Default|GetHitRight) (not (Variables|Default|GetHitLeft)) (not (Variables|Default|GetHitUp)))
      (Transformation|AddRelativeRotation (Variables|Default|GetDecal) "45.000000,40.000000,0.000000" false false)
      (Development|PrintString "HitDownRight")
      (elif (Math|Boolean|ANDBoolean (Variables|Default|GetHitDown) (not (Variables|Default|GetHitRight)) (Variables|Default|GetHitLeft) (not (Variables|Default|GetHitUp)))
        (Transformation|AddRelativeRotation (Variables|Default|GetDecal) "45.000000,-40.000000,0.000000" false false)
        (Development|PrintString "HitDownLeft")
        (elif (Math|Boolean|ANDBoolean (not (Variables|Default|GetHitDown)) (not (Variables|Default|GetHitRight)) (not (Variables|Default|GetHitLeft)) (Variables|Default|GetHitUp))
          (Transformation|AddRelativeRotation (Variables|Default|GetDecal) "-40.000000,0.000000,0.000000" false false)
          (elif (Math|Boolean|ANDBoolean (not (Variables|Default|GetHitDown)) (not (Variables|Default|GetHitRight)) (Variables|Default|GetHitLeft) (Variables|Default|GetHitUp))
            (Transformation|AddRelativeRotation (Variables|Default|GetDecal) "40.000000,-35.000000,0.000000" false false)
            (elif (Math|Boolean|ANDBoolean (not (Variables|Default|GetHitDown)) (Variables|Default|GetHitRight) (not (Variables|Default|GetHitLeft)) (Variables|Default|GetHitUp))
              (Transformation|AddRelativeRotation (Variables|Default|GetDecal) "40.000000,35.000000,0.000000" false false)
              (elif (Math|Boolean|ANDBoolean (not (Variables|Default|GetHitDown)) (Variables|Default|GetHitRight) (not (Variables|Default|GetHitLeft)) (not (Variables|Default|GetHitUp)))
                (Transformation|AddRelativeRotation (Variables|Default|GetDecal) "-35.000000,0.000000,0.000000" false false)
                (elif (Math|Boolean|ANDBoolean (not (Variables|Default|GetHitDown)) (not (Variables|Default|GetHitRight)) (Variables|Default|GetHitLeft) (not (Variables|Default|GetHitUp)))
                  (Transformation|AddRelativeRotation (Variables|Default|GetDecal) "35.000000,0.000000,0.000000" false false))))))))))

(event EventBeginPlay
  (Utilities|FlowControl|Delay 0.2)
  (bind _returnvalue (Rendering|Material|CreateDynamicMaterialInstance (Variables|Default|GetMaterialInstance) "None" "None" :!class /Script/Engine.KismetMaterialLibrary))
  (Rendering|Components|Decal|SetDecalMaterial (Variables|Default|GetDecal) _returnvalue)
  (Variables|Default|SetDynamicDecal _returnvalue)
  (Variables|Default|GetShot?
    (:then
      (bind _hitsurface_ (CallFunction|LineTrace (Variables|Default|GetDown)))
      (Variables|Default|SetHitDown _hitsurface_)
      (bind _hitsurface__2 (CallFunction|LineTrace (Variables|Default|GetLeft)))
      (Variables|Default|SetHitLeft _hitsurface__2)
      (bind _hitsurface__3 (CallFunction|LineTrace (Variables|Default|GetRight)))
      (Variables|Default|SetHitRight _hitsurface__3)
      (bind _hitsurface__4 (CallFunction|LineTrace (Variables|Default|GetUp)))
      (Variables|Default|SetHitUp _hitsurface__4)
      (CallFunction|SetRotation))
    (:else)))

(event EventClean
  (bind _transition (Timeline|Timeline PlayFromStart)
    (:Update
      (Variables|Default|SetNewDissolve (Math|Float|Lerp (Variables|Default|GetDissolveStart) (+ (Variables|Default|GetDissolveStart) (Variables|Default|GetRemoveVariable)) _transition)))
    (:Finished
      (Variables|Default|SetDissolveStart (+ (Variables|Default|GetDissolveStart) (Variables|Default|GetRemoveVariable))))))

(fn ConstructionScript)

(fn LineTrace
  (params (Arrow :type Arrow%20Component%20Object%20Reference))
  (bind _returnvalue (Transformation|GetWorldLocation Arrow))
  (bind _returnvalue_2 (Collision|LineTraceForObjects _returnvalue (+ _returnvalue (* (Math|Vector|GetForwardVector Arrow) 2e+02)) (Utilities|Array|MakeArray "ObjectTypeQuery1") false 0 "ForDuration"))
  (return _returnvalue_2))

(fn OnRepNewDissolve
  (Rendering|Material|SetScalarParameterValue (Variables|Default|GetDynamicDecal) "Dissolve" (Variables|Default|GetNewDissolve) :!class /Script/Engine.MaterialInstanceDynamic))

(fn GetEquipmentHealth
  (return 0.0))

(fn GetEquipmentType
  (params (PlayerAsking :type BP%20First%20Person%20Character%20Object%20Reference))
  (return "NewEnumerator5"))