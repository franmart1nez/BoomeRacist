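; BP_DirtDirector gathers every BP_Dirt actor in the level and activates those belonging to the first floor.
; After a short delay on BeginPlay it caches the actors, prints the count, then activates each one whose first tag is Floor1.
; The 0 key re-runs the activation loop, and the ActivateFloor event exists but is empty, so the floor number is fixed.
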(event Custom|ActivateFloor
  (params (FloorNumber :type Integer)))

(event EventBeginPlay
  (Utilities|FlowControl|Delay 0.2)
  (bind _outactors (Actor|GetAllActorsOfClass "/Game/Programming/Cleaning/BP_Dirt.BP_Dirt_C"))
  (bind _output_get (Variables|Default|SetAllDirt _outactors))
  (Development|PrintString (Utilities|String|ToString(Integer) (Utilities|Array|Length _output_get)))
  (for _array_element (Variables|Default|GetAllDirt)
    (if (== (Utilities|Array|Get(acopy) (Variables|/Script/Engine.Actor|GetTags _array_element)) (Utilities|String|StringToName (Utilities|String|Append "Floor" "1")))
      (Default|Activate _array_element))))

(event Input|KeyboardEvents|0
  (params (Key :type Key%20Structure :default "None"))
  (:Pressed
    (for _array_element (Variables|Default|GetAllDirt)
      (if (== (Utilities|Array|Get(acopy) (Variables|/Script/Engine.Actor|GetTags _array_element)) (Utilities|String|StringToName (Utilities|String|Append "Floor" "1")))
        (Default|Activate _array_element)))))

(fn ConstructionScript)