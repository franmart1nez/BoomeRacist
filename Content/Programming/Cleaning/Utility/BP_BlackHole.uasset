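; Black hole actor that pulls in physics-simulating objects, shrinks them and destroys them with a suck sound near its center.
; AttractionExtent overlaps store components with their original damping and scale, grouped by actor, and enable Tick.
; Tick applies stronger force and damping inside NoReturnExtent, while material parameters drive stretching sized by StretchExtent.
; End overlap passes its own sphere, not OtherComp, to RemoveStoredComponent, so restoration never matches.
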(event OnComponentBeginOverlap(AttractionExtent)
  (params (OverlappedComponent :type Primitive%20Component%20Object%20Reference) (OtherActor :type Actor%20Object%20Reference) (OtherComp :type Primitive%20Component%20Object%20Reference) (OtherBodyIndex :type Integer) (bFromSweep :type Boolean) (SweepResult :type Hit%20Result%20Structure%20%28by%20ref%29))
  ;[0.15 0.15 0.15 0.5] First Overlap (AttractionExtent)
  ;[0.15 0.15 0.15 0.5] Store Actor
  (if (Physics|IsSimulatingPhysics OtherComp "None")
    (Actor|Tick|SetActorTickEnabled true)
    (CallFunction|StoreComponent OtherComp OtherActor)
    ;[0.15 0.15 0.15 0.5] Set stretch effect in Material
    (bind _asmesh_component (Utilities|Casting|CastToMeshComponent OtherComp))
    (Rendering|Material|SetVectorParameterValueonMaterials _asmesh_component "CustomStretchPosition" (Transformation|GetWorldLocation (Variables|Default|GetNoReturnExtent)))
    (Rendering|Material|SetScalarParameterValueonMaterials _asmesh_component "StretchActivated" 1.0)
    (Rendering|Material|SetScalarParameterValueonMaterials _asmesh_component "Radius" (Components|Sphere|GetScaledSphereRadius (Variables|Default|GetStretchExtent)))))

(event OnComponentBeginOverlap(NoReturnExtent)
  (params (OverlappedComponent :type Primitive%20Component%20Object%20Reference) (OtherActor :type Actor%20Object%20Reference) (OtherComp :type Primitive%20Component%20Object%20Reference) (OtherBodyIndex :type Integer) (bFromSweep :type Boolean) (SweepResult :type Hit%20Result%20Structure%20%28by%20ref%29))
  ;[0.15 0.15 0.15 0.5] Destroy when near center
)

(event OnComponentEndOverlap(AttractionExtent)
  (params (OverlappedComponent :type Primitive%20Component%20Object%20Reference) (OtherActor :type Actor%20Object%20Reference) (OtherComp :type Primitive%20Component%20Object%20Reference) (OtherBodyIndex :type Integer))
  ;[0.15 0.15 0.15 0.5] Leaves Attraction Range
  (CallFunction|RemoveStoredComponent OverlappedComponent OtherActor)
  (if (Utilities|Array|IsEmpty (Variables|Default|GetAffectedActorsArray))
    (Actor|Tick|SetActorTickEnabled false)))

(event Custom|Destroy
  (params (ComponentAttracted :type Primitive%20Component%20Object%20Reference) (ActorAttracted :type Actor%20Object%20Reference))
  ;[0.15 0.15 0.15 0.5] Destroy when near center
  (CallFunction|RemoveStoredComponent ComponentAttracted ActorAttracted)
  (Actor|DestroyActor ActorAttracted))

(event EventBeginPlay)

(event EventTick
  (params (DeltaSeconds :type Float%20%28single-precision%29))
  (if (Utilities|Array|IsNotEmpty (Variables|Default|GetAffectedActorsArray))
    (CallFunction|AttractActor)
    (CallFunction|DestroyComponent)))

(fn ConstructionScript)

(fn StoreComponent
  (params (Component :type Primitive%20Component%20Object%20Reference) (Actor :type Actor%20Object%20Reference))
  (bind _affectedactorsarray (Variables|Default|GetAffectedActorsArray))
  (LocalVariables|SetL_AffectedComponent (Utilities|Struct|MakeSTR_BlackHoleComponents Component (Class|PrimitiveComponent|GetLinearDamping Component) (Class|PrimitiveComponent|GetAngularDamping Component) (Transformation|GetWorldScale Component)))
  (LocalVariables|SetL_OverlappedActor Actor)
  (for (_array_element _array_index) _affectedactorsarray
    (Development|PrintString "add to existing")
    (if (== (LocalVariables|GetL_OverlappedActor) (.Actor (Utilities|Struct|BreakSTR_BlackHoleActors _array_element)))
      (Utilities|Array|Add (.AffectedComponents (Utilities|Struct|BreakSTR_BlackHoleActors (Utilities|Array|Get(acopy) _affectedactorsarray _array_index))) (LocalVariables|GetL_AffectedComponent))
      (LocalVariables|SetL_FoundActor? true)))
  (if (not (LocalVariables|GetL_FoundActor?))
    (Utilities|Array|Add (Variables|Default|GetAffectedActorsArray) (Utilities|Struct|MakeSTR_BlackHoleActors (LocalVariables|GetL_OverlappedActor) (Utilities|Array|MakeArray (LocalVariables|GetL_AffectedComponent)) (Transformation|GetActorScale3D (LocalVariables|GetL_OverlappedActor))))
    (Development|PrintString "add new")))

(fn AttractActor
  (bind _noreturnextent (Variables|Default|GetNoReturnExtent))
  (bind _returnvalue (Components|Sphere|GetScaledSphereRadius _noreturnextent))
  ;[1 1 1] Go through the list of registered components
  (for _array_element (Variables|Default|GetAffectedActorsArray)
    (if (Utilities|IsValid (.Actor (Utilities|Struct|BreakSTR_BlackHoleActors _array_element)))
      (LocalVariables|SetParentActor (.Actor (Utilities|Struct|BreakSTR_BlackHoleActors _array_element)))
      (for _array_element_2 (.AffectedComponents (Utilities|Struct|BreakSTR_BlackHoleActors _array_element))
        (LocalVariables|SetAttractedComponent (.component _array_element_2))
        (LocalVariables|SetDirectionTowardsCenter (Math|Vector|Normalize (- (Transformation|GetWorldLocation (Variables|Default|GetAttractionExtent)) (Transformation|GetWorldLocation (LocalVariables|GetAttractedComponent)))))
        (LocalVariables|SetDistanceToCenter (Math|Vector|VectorLength (- (Transformation|GetWorldLocation (Variables|Default|GetAttractionExtent)) (Transformation|GetWorldLocation (LocalVariables|GetAttractedComponent)))))
        (LocalVariables|SetIsEnveloped (< (LocalVariables|GetDistanceToCenter) _returnvalue))
        (Transformation|SetActorScale3D (LocalVariables|GetParentActor) (* (.InitialScale (Utilities|Struct|BreakSTR_BlackHoleActors _array_element)) (Math|Float|Clamp(Float) (/ (LocalVariables|GetDistanceToCenter) _returnvalue))))
        ;[1 1 1] Add damping to object's movement (this should be done on entering)
        (Class|PrimitiveComponent|SetLinearDamping (LocalVariables|GetAttractedComponent) (select (LocalVariables|GetIsEnveloped) (Variables|Default|GetEnvelopedDamping) 0.1))
        (Class|PrimitiveComponent|SetAngularDamping (LocalVariables|GetAttractedComponent) (select (LocalVariables|GetIsEnveloped) (Variables|Default|GetEnvelopedDamping) 0.1))
        (Physics|AddForce (LocalVariables|GetAttractedComponent) (* (LocalVariables|GetDirectionTowardsCenter) (select (LocalVariables|GetIsEnveloped) (Variables|Default|GetEnvelopedForce) (Variables|Default|GetAttractionFoce))) "None" false)
        ;[1 1 1] Setting the stretch extent of the black hole.
        ; This has to be done each frame in order to take into account the black hole scaling up and down.
        (bind _asmesh_component (Utilities|Casting|CastToMeshComponent (LocalVariables|GetAttractedComponent)))
        (Rendering|Material|SetScalarParameterValueonMaterials _asmesh_component "Radius" (Components|Sphere|GetScaledSphereRadius (Variables|Default|GetStretchExtent)))))))

(fn RemoveStoredComponent
  (params (ComponentAttracted :type Primitive%20Component%20Object%20Reference) (ActorAttracted :type Actor%20Object%20Reference))
  (for (_array_element _array_index) (Variables|Default|GetAffectedActorsArray)
    (if (== (.Actor (Utilities|Struct|BreakSTR_BlackHoleActors _array_element)) ActorAttracted)
      (for (_array_element_2 _array_index_2) (.AffectedComponents (Utilities|Struct|BreakSTR_BlackHoleActors _array_element))
        (if (== ComponentAttracted (.Component (Utilities|Struct|BreakSTR_BlackHoleComponents _array_element_2)))
          (Utilities|FlowControl|Sequence
            (:then_0
              ;[0.15 0.15 0.15 0.5] Return Phys settings
              (Class|PrimitiveComponent|SetLinearDamping ComponentAttracted (.LinearDamping (Utilities|Struct|BreakSTR_BlackHoleComponents _array_element_2)))
              (Class|PrimitiveComponent|SetAngularDamping ComponentAttracted (.AngularDamping (Utilities|Struct|BreakSTR_BlackHoleComponents _array_element_2)))
              (Transformation|SetWorldScale3D ComponentAttracted (.OriginalScale (Utilities|Struct|BreakSTR_BlackHoleComponents _array_element_2))))
            (:then_1
              ;[0.15 0.15 0.15 0.5] Deactivate Stretch in Material
              (bind _asstatic_mesh_component (Utilities|Casting|CastToStaticMeshComponent ComponentAttracted))
              (Rendering|Material|SetScalarParameterValueonMaterials _asstatic_mesh_component "StretchActivated" 0.0))
            (:then_2
              (Utilities|Array|RemoveIndex (.AffectedComponents (Utilities|Struct|BreakSTR_BlackHoleActors (Utilities|Array|Get(acopy) (Variables|Default|GetAffectedActorsArray) _array_index))) _array_index_2)
              (if (Utilities|Array|IsEmpty (.AffectedComponents (Utilities|Struct|BreakSTR_BlackHoleActors (Utilities|Array|Get(acopy) (Variables|Default|GetAffectedActorsArray) _array_index))))
                (Utilities|Array|RemoveIndex (Variables|Default|GetAffectedActorsArray) _array_index)))))))))

(fn DestroyComponent
  (for (_array_element _array_index) (Variables|Default|GetAffectedActorsArray)
    (for _array_element_2 (.AffectedComponents (Utilities|Struct|BreakSTR_BlackHoleActors _array_element))
      (if (< (/ (Math|Vector|VectorLength (- (Transformation|GetWorldLocation (Variables|/Script/Engine.Actor|GetRootComponent (.Actor (Utilities|Struct|BreakSTR_BlackHoleActors _array_element)))) (Transformation|GetWorldLocation (Variables|Default|GetNoReturnExtent)))) (Components|Sphere|GetScaledSphereRadius (Variables|Default|GetNoReturnExtent))) 0.5)
        (Actor|DestroyActor (.Actor (Utilities|Struct|BreakSTR_BlackHoleActors _array_element)))
        (Audio|PlaySoundatLocation "/Game/Programming/Sounds/Misc/DarkHole_SUCK.DarkHole_SUCK" (Transformation|GetActorLocation) "0, 0, 0" 1.0 1.0 0.0 0 0 0 0)
        (Utilities|Array|RemoveIndex (Variables|Default|GetAffectedActorsArray) _array_index))))
  (return))