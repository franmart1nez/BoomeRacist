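; BP_Chicken is an AI-driven chicken that also acts as equipment, running BT_Chicken once possessed by BP_AI_Chicken.
; Enable/DisablePhysics switches between AI control and physics on the capsule and the mesh bodies below the base bone.
; Unequip waits briefly, stops physics, lerps the capsule rotation back to zero with a timeline, then re-enables the AI.
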(event EventBeginPlay)

(event Collision|EventActorBeginOverlap
  (params (OtherActor :type Actor%20Object%20Reference)))

(event EventTick
  (params (DeltaSeconds :type Float%20%28single-precision%29)))

(event EventPossessed
  (params (NewController :type Controller%20Object%20Reference))
  (bind _asbp_ai_chicken (Utilities|Casting|CastToBP_AI_Chicken NewController))
  (bind _output_get (Variables|Default|SetAIControllerChicken _asbp_ai_chicken))
  (AI|RunBehaviorTree _output_get "/Game/Programming/Cleaning/Chicken/BT_Chicken.BT_Chicken"))

(event EventEnable/DisablePhysics
  (params (Enable? :type Boolean))
  (Default|Enable/DisableAI (Variables|Default|GetAIControllerChicken) (not Enable?))
  (Physics|SetSimulatePhysics (Variables|Collision|GetCapsuleComponent) Enable?)
  (Class|SkeletalMeshComponent|SetAllBodiesBelowSimulatePhysics (Variables|Character|GetMesh) (Utilities|Name|MakeLiteralName "base") true false)
  (if (not Enable?)
    (Collision|SetCollisionResponsetoChannel (Variables|Collision|GetCapsuleComponent) "ECC_Pawn" (select Enable? "ECR_Block" "ECR_Ignore"))))

(event EventUnequip
  (params (Force :type Vector :default "0, 0, 0"))
  (Utilities|FlowControl|Delay 3.5)
  (Class|SkeletalMeshComponent|SetAllBodiesBelowSimulatePhysics (Variables|Character|GetMesh) (Utilities|Name|MakeLiteralName "base") false true)
  (Physics|SetSimulatePhysics (Variables|Collision|GetCapsuleComponent) false)
  (Variables|Default|SetRotisseryChicken (Transformation|GetWorldRotation (Variables|Collision|GetCapsuleComponent)))
  (bind _rotate (Timeline|Rotation%20Lerp PlayFromStart)
    (:Update
      (Development|PrintString (Utilities|String|ToString(Float) _rotate))
      (Transformation|SetWorldRotation (Variables|Collision|GetCapsuleComponent) (Math|Rotator|Lerp(Rotator) (Variables|Default|GetRotisseryChicken) "0, 0, 0" _rotate) false false))
    (:Finished
      (Default|Enable/DisableAI (Variables|Default|GetAIControllerChicken) true))))

(fn ConstructionScript)

(fn GetEquipmentType
  (params (PlayerAsking :type BP%20First%20Person%20Character%20Object%20Reference))
  (return "NewEnumerator1"))