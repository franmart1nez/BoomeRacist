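; BP_Dirt is a cleanable dirt decal for the cleaning gameplay.
; Half a second after BeginPlay it puts a dynamic material on the decal.
; Clean raises replicated Opacity until Cleaned is set; OnRep_Opacity drives the Dissolve parameter and sets Cleaned at a low threshold, despite the increasing value.
; WetWindows only sets IsWet, and the equipment getters return fixed values.
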(event Custom|Activate
  (Utilities|FlowControl|Delay 0.5)
  (bind _returnvalue (Rendering|Material|CreateDynamicMaterialInstance (Variables|Default|GetMaterialInstace) "None" "None" :!class /Script/Engine.KismetMaterialLibrary))
  (bind _output_get (Variables|Default|SetDynamicMI _returnvalue))
  (Rendering|Components|Decal|SetDecalMaterial (Variables|Default|GetDecal) _output_get))

(event EventBeginPlay
  (CallFunction|Activate))

(event EventWetWindows
  (Variables|Default|SetIsWet? true))

(event EventClean
  (if (not (Variables|Default|GetCleaned?))
    (Variables|Default|SetOpacity (+ (Variables|Default|GetOpacity) 0.05))))

(fn ConstructionScript)

(fn OnRepOpacity
  (bind _opacity (Variables|Default|GetOpacity))
  (Rendering|Material|SetScalarParameterValue (Variables|Default|GetDynamicMI) "Dissolve" _opacity :!class /Script/Engine.MaterialInstanceDynamic)
  (if (<= _opacity 0.1)
    (Variables|Default|SetCleaned? true)))

(fn GetEquipmentHealth
  (return 0.0))

(fn GetEquipmentType
  (params (PlayerAsking :type BP%20First%20Person%20Character%20Object%20Reference))
  (return "NewEnumerator5"))