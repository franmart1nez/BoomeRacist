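; BP_Tragaperras is an interactable slot machine that always makes the player lose.
; Its interact event charges a fixed fee from the cached first-person character's Money, if affordable, and refreshes the character's widget.
; It briefly shows a WDG_YOULOSE widget, then raises the Gambling stat after the delay.
; An IsLosing flag blocks repeat interaction while the losing sequence runs.
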(event EventGamble/Drink/Interact
  (bind _as_bp_first_person_character (Variables|Default|GetAs%20BP%20First%20Person%20Character))
  (bind _as_bp_first_person_character_2 (Variables|Default|GetAs%20BP%20First%20Person%20Character))
  (if (not (Variables|Default|GetIsLosing?))
    (if (not (< (Variables|/Game/FirstPerson/Blueprints/BP_FirstPersonCharacter.BP_FirstPersonCharacter_C|GetMoney _as_bp_first_person_character) 3.0))
      (Variables|/Game/FirstPerson/Blueprints/BP_FirstPersonCharacter.BP_FirstPersonCharacter_C|SetMoney _as_bp_first_person_character (- (Variables|/Game/FirstPerson/Blueprints/BP_FirstPersonCharacter.BP_FirstPersonCharacter_C|GetMoney _as_bp_first_person_character) 3.0))
      (Default|UpdateWidget _as_bp_first_person_character)
      (Variables|Default|SetIsLosing? true)
      (bind _returnvalue (UserInterface|CreateWidget "/Game/Programming/Widgets/WDG_YOULOSE.WDG_YOULOSE_C"))
      (bind _output_get (Variables|Default|Setwidget _returnvalue))
      (UserInterface|Viewport|AddtoViewport _output_get 0)
      (Utilities|FlowControl|Delay 1.0)
      (Variables|/Game/FirstPerson/Blueprints/BP_FirstPersonCharacter.BP_FirstPersonCharacter_C|SetGambling _as_bp_first_person_character_2 (+ (Variables|/Game/FirstPerson/Blueprints/BP_FirstPersonCharacter.BP_FirstPersonCharacter_C|GetGambling _as_bp_first_person_character_2) 1e+01))
      (Widget|RemovefromParent (Variables|Default|Getwidget))
      (Variables|Default|SetIsLosing? false))))

(event EventBeginPlay
  (bind _asbp_first_person_character (Utilities|Casting|CastToBP_FirstPersonCharacter (Game|Player|GetPlayerPawn 0)))
  (Variables|Default|SetAs%20BP%20First%20Person%20Character _asbp_first_person_character))

(fn ConstructionScript)