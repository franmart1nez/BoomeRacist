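; BP_Matress is the interactable mattress that ends the day, restoring player health, lowering Alcohol and Gambling, and advancing the day counter.
; Each interaction refreshes the player HUD, shows a day announcement widget (also shown on BeginPlay) and has BP_DirtDirector choose that day's floors.
; After day 2 it disables all elevators; after day 3 it also calls the hostility update on every enemy walker, nested inside the elevator loop.
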(event Custom|NewDay
  (bind _returnvalue (UserInterface|CreateWidget "/Game/Programming/Widgets/WDG_DayAnnouncemnt.WDG_DayAnnouncemnt_C"))
  (bind _output_get (Variables|Default|SetDayWidget _returnvalue))
  (Default|SetDayh _output_get (Utilities|Text|ToText(String) (Utilities|String|Append "Day " (Utilities|String|ToString(Integer) (Variables|/Game/FirstPerson/Blueprints/BP_FirstPersonCharacter.BP_FirstPersonCharacter_C|GetDayNumber (Variables|Default|GetAs%20BP%20First%20Person%20Character))))))
  (UserInterface|Viewport|AddtoViewport _output_get 0))

(event EventBeginPlay
  (bind _asbp_first_person_character (Utilities|Casting|CastToBP_FirstPersonCharacter (Game|Player|GetPlayerPawn 0)))
  (Variables|Default|SetAs%20BP%20First%20Person%20Character _asbp_first_person_character)
  (CallFunction|NewDay))

(event EventGamble/Drink/Interact
  (bind _as_bp_first_person_character (Variables|Default|GetAs%20BP%20First%20Person%20Character))
  (Variables|/Game/FirstPerson/Blueprints/BP_FirstPersonCharacter.BP_FirstPersonCharacter_C|SetHealth _as_bp_first_person_character 1e+02)
  (Math|Integer|IncrementInt (Variables|/Game/FirstPerson/Blueprints/BP_FirstPersonCharacter.BP_FirstPersonCharacter_C|GetDayNumber _as_bp_first_person_character)
    (:%20%20
      (Variables|/Game/FirstPerson/Blueprints/BP_FirstPersonCharacter.BP_FirstPersonCharacter_C|SetAlcohol _as_bp_first_person_character (- (Variables|/Game/FirstPerson/Blueprints/BP_FirstPersonCharacter.BP_FirstPersonCharacter_C|GetAlcohol _as_bp_first_person_character) 2e+01))
      (Variables|/Game/FirstPerson/Blueprints/BP_FirstPersonCharacter.BP_FirstPersonCharacter_C|SetGambling _as_bp_first_person_character (- (Variables|/Game/FirstPerson/Blueprints/BP_FirstPersonCharacter.BP_FirstPersonCharacter_C|GetGambling _as_bp_first_person_character) 2e+01))
      (Default|UpdateWidget _as_bp_first_person_character)
      (CallFunction|NewDay)
      (bind _returnvalue (Actor|GetActorOfClass "/Game/Programming/Cleaning/BP_DirtDirector.BP_DirtDirector_C"))
      (Default|ChooseFloorsforDay _returnvalue)
      (if (> (Variables|/Game/FirstPerson/Blueprints/BP_FirstPersonCharacter.BP_FirstPersonCharacter_C|GetDayNumber (Variables|Default|GetAs%20BP%20First%20Person%20Character)) 2)
        (bind _outactors (Actor|GetAllActorsOfClass "/Game/Programming/Elevator/BP_Elevator.BP_Elevator_C"))
        (for _array_element _outactors
          (Default|Disable _array_element)
          (if (> (Variables|/Game/FirstPerson/Blueprints/BP_FirstPersonCharacter.BP_FirstPersonCharacter_C|GetDayNumber (Variables|Default|GetAs%20BP%20First%20Person%20Character)) 3)
            (bind _outactors_2 (Actor|GetAllActorsOfClass "/Game/Programming/Enemies/Characters(legacy)/BP_BaseEnemyWalker.BP_BaseEnemyWalker_C"))
            (for _array_element_2 _outactors_2
              (Default|UPDATEhOSTILE _array_element_2))))))))

(fn ConstructionScript)