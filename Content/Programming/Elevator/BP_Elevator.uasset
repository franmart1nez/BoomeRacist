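; BP_Elevator is an elevator that moves the player between floors by teleporting them to another elevator.
; Interacting while active opens a WDG_ElevatorNumber widget in UI-only input with a cursor, passing itself as owner.
; Teleport matches the floor number against the first tag of elevators gathered shortly after BeginPlay, moves the pawn, then restores game input.
; Disable deactivates the elevator and shows a blocking barrier.
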(event Custom|Teleport
  (params (FloorNumber :type Name))
  (bind _returnvalue (Game|GetPlayerController 0))
  (bind _array_element (Utilities|Array|ForEachLoopwithBreak (Variables|Default|GetElevators) :!label _label)
    (:LoopBody
      (if (== (Utilities|Array|Get(acopy) (Variables|/Script/Engine.Actor|GetTags _array_element)) FloorNumber)
        (Transformation|SetActorLocation (Game|Player|GetPlayerPawn 0) (Transformation|GetActorLocation _array_element) false true)
        (goto _label Break)))
    (:Completed
      (Widget|RemovefromParent (Variables|Default|GetElevatorWidget))
      (Input|SetInputModeGameOnly _returnvalue false)
      (Variables|/Script/Engine.PlayerController|SetbShowMouseCursor _returnvalue false))))

(event Custom|Disable
  (Variables|Default|SetActive? false)
  (Rendering|SetVisibility (Variables|Default|GetBarrier) true false)
  (Collision|SetCollisionResponsetoAllChannels (Variables|Default|GetBarrier) "ECR_Block"))

(event EventBeginPlay
  (Utilities|FlowControl|Delay 0.2)
  (bind _outactors (Actor|GetAllActorsOfClass "BP_Elevator_C"))
  (Variables|Default|SetElevators _outactors))

(event Collision|EventActorBeginOverlap
  (params (OtherActor :type Actor%20Object%20Reference)))

(event EventTick
  (params (DeltaSeconds :type Float%20%28single-precision%29)))

(event EventGamble/Drink/Interact
  (bind _returnvalue (Game|GetPlayerController 0))
  (if (Variables|Default|GetActive?)
    (Input|SetInputModeUIOnly _returnvalue 0 "DoNotLock" false)
    (Variables|/Script/Engine.PlayerController|SetbShowMouseCursor _returnvalue true)
    (bind _returnvalue_2 (UserInterface|CreateWidget "/Game/Programming/Widgets/WDG_ElevatorNumber.WDG_ElevatorNumber_C" 0 self))
    (bind _output_get (Variables|Default|SetElevatorWidget _returnvalue_2))
    (UserInterface|Viewport|AddtoViewport _output_get 0)))

(fn ConstructionScript)